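; Mortar Blueprint, an aimed enemy or emplacement with a turret, barrel and health bar.
; On BeginPlay it initializes its TankAiming component with the TankBarrel and TankTurret parts.
; It then passes itself to the MortarHealthBar user widget on its Widget component as that bar's mortar reference.
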(event `self.ReceiveBeginPlay`
  (`TankAimingComponent.Initialize` (`self.TankAiming`) (`self.TankBarrel`) (`self.TankTurret`))
  (`self.InitializeHealthBarWidget`))

(fn `InitializeHealthBarWidget`
  (set `/Game/UI/MortarHealthBar.MortarReference` self (cast `/Game/UI/MortarHealthBar` (`WidgetComponent.GetUserWidgetObject` (`self.Widget`)) :!pure true)))

(fn `UserConstructionScript`)